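; Game mode for a defusal match that times an opening buy phase.
; BeginPlay starts a timer that calls End Buy Phase, which finds the BP_Barrier actors and destroys them if the first is valid.
; Play Phase is an unfinished stub: its timer names no function, it adds zero to its duration, and nothing here calls it.
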(event `self.ReceiveBeginPlay`
  (`KismetSystemLibrary.K2_SetTimer` null "End Buy Phase" (`self.Buy phase time`)))

(fn `End Buy Phase`
  (bind _outactors (`GameplayStatics.GetAllActorsOfClass` "/Game/Core/Blueprints/Prefabs/BP_Barrier.BP_Barrier_C"))
  (`/Engine/EditorBlueprintResources/StandardMacros.IsValid` (`|GetArrayItem` _outactors)
    (:`Is Valid`
      (`self.K2_DestroyActor` _outactors))))

(fn `Play Phase`
  (`KismetSystemLibrary.K2_SetTimer` null "" (`self.Play phase time`))
  (set `self.Play phase time` (+ (`self.Play phase time`) 0.0)))

(fn `UserConstructionScript`)