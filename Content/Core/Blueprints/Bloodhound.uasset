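; Bloodhound character Blueprint that triggers a temporary speed-boost ultimate when X is pressed.
; The key press sends an ultimate request to the CAbilityFrameWork component, then doubles walk speed through CharacterMovement without checking the request's outcome.
; A two-second one-shot timer restores the slower walk speed and resets the ultimate in the ability framework.
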(event `Key|X`
  (params (Key :type "Key Structure"))
  (:`Pressed`
    (`/Game/Core/Blueprints/Scripts/C_Ability_FrameWork.Request ULT` (`self.C_Ability_FrameWork`) 0.01 false)
    (`self.Speed Baire Jabi`)))

(event `Speed Baire Jabi`
  (set `CharacterMovementComponent.MaxWalkSpeed` 1200.0 (`self.CharacterMovement`))
  (`KismetSystemLibrary.K2_SetTimerDelegate` (delegate `Reset`) 2.0))

(event `Reset`
  (set `CharacterMovementComponent.MaxWalkSpeed` 600.0 (`self.CharacterMovement`))
  (`/Game/Core/Blueprints/Scripts/C_Ability_FrameWork.Reset ULT` (`self.C_Ability_FrameWork`)))

(fn `UserConstructionScript`
  (`parent.UserConstructionScript`))