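; Character component that tracks health and alive state, with unfinished scaffolding for an ultimate (ULT) ability.
; Init stores the owning character reference, and ChangeHealth refreshes the alive flag before applying a clamped delta, only while alive.
; ULT helpers set timers by function name, but the charge and reset functions are empty, the request check never passes, and the charge timer's name mismatches its function.
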(event `Init Health Component`
  (params (Charachter :type "/Game/Core/Blueprints/Base_Charachter Object Reference"))
  ;[0 0 0] Begin Play
  (set `self.Reference Charachter` Charachter))

(fn `Calculate ULT charges`)

(fn `Change Health`
  (params (`Change Ammount` :type "Float (double-precision)"))
  (`self.Check Alive`)
  (if (`self.Is Alive`)
    (set `self.Current Health` (`KismetMathLibrary.FClamp` (+ (`self.Current Health`) `Change Ammount`) 0.0 100.0))))

(fn `Check Alive`
  (if (== (`self.Current Health`) 0.0)
    (set `self.Is Alive` false)
    (else
      (set `self.Is Alive` true))))

(fn `Request ULT`
  (params (`Start Offset` :type "Float (single-precision)") (Condition :type Boolean))
  (if (== 0 100)
    (if Condition
      (`KismetSystemLibrary.K2_SetTimer` null "Reset ULT" `Start Offset`))))

(fn `Reset ULT`)

(fn `Start Ult Timer`
  (params (Time :type "Float (single-precision)") (bLooping :type Boolean))
  (`KismetSystemLibrary.K2_SetTimer` null "Calculate Charges " Time bLooping))