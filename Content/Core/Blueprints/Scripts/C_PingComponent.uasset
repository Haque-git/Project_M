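; C_PingComponent is a character component that places a ping marker in the world where the player looks.
; RequestPing line-traces from the character's camera on the Visibility channel and spawns a BP_Ping at the impact point.
; A looping timer of PingLifespan then destroys every actor of the last ping's class, not just that one.
; The character reference arrives through InitHealthComponent, despite its name.
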(event `Init Health Component`
  (params (Charachter :type "/Game/Core/Blueprints/Base_Charachter Object Reference"))
  ;[0 0 0] Begin Play
  (set `self.Reference Charachter` Charachter))

(event `Request Ping`
  (`self.Use Ping`)
  (`KismetSystemLibrary.K2_SetTimerDelegate` (delegate `Destroy Ping`) (`self.Ping Lifespan`) true))

(event `Destroy Ping`
  (bind _outactors (`GameplayStatics.GetAllActorsOfClass` (`GameplayStatics.GetObjectClass` (`self.Ping Actor`))))
  (`/Game/Core/Blueprints/Prefabs/Miscs/BP_Ping.Destroy ` _outactors))

(fn `Trace For Interaction`
  (returns (Result :type Boolean) (OutHit :type "HitResult Structure"))
  (bind _camera (`/Game/Core/Blueprints/Base_Charachter.Camera` (`self.Reference Charachter`)))
  (bind _returnvalue (`SceneComponent.K2_GetComponentLocation` _camera))
  (bind (_outhit _returnvalue_2) (`KismetSystemLibrary.LineTraceSingle` _returnvalue (+ _returnvalue (* (`SceneComponent.GetForwardVector` _camera) 10000.0)) "TraceTypeQuery1"))
  (return _returnvalue_2 _outhit))

(fn `Use Ping`
  (returns (`Ping Actor` :type "/Game/Core/Blueprints/Prefabs/Miscs/BP_Ping Object Reference") (HitActor :type "Actor Object Reference"))
  (bind (_result _outhit) (`self.Trace For Interaction`))
  (if _result
    (bind (_bblockinghit _binitialoverlap _time _distance _location _impactpoint _normal _impactnormal _physmat _hitactor) (`GameplayStatics.BreakHitResult` _outhit))
    (bind _returnvalue (`|SpawnActorFromClass` "/Game/Core/Blueprints/Prefabs/Miscs/BP_Ping.BP_Ping_C" (`KismetMathLibrary.MakeTransform` _impactpoint) "Undefined" "OverrideRootScale" null null))
    (bind _output_get (set `self.Ping Actor` _returnvalue))
    (return _output_get _hitactor)))