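; Ability component that manages a character's ultimate charge and tactical ability charges.
; Init starts a looping timer that fills ultimate charge to 100, and RequestULT can reset it after a delay when full.
; CanUse, gated by a toggle enum, spends a tactical charge and starts a looping recharge timer if one was available.
; Helpers lerp camera FOV from its default and print both charges on Tick when debugging.
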(event `self.ReceiveTick`
  (params (DeltaSeconds :type "Float (single-precision)"))
  ;[0.8177 0.08092 0.08092] Debug
  (if (`self.bDebugInfo`)
    (`self.Start Debug` "X")))

(event `Init Ability Component`
  (params (Charachter :type "/Game/Core/Blueprints/Base_Charachter Object Reference"))
  ;[0 0 0] Begin Play
  (set `self.Reference Charachter` Charachter)
  (`self.Start Ult Timer` 0.3 true))

(fn `Calculate ULT charges`
  (set `self.Current Charge ULT` (`KismetMathLibrary.Clamp` (+ (`self.Current Charge ULT`) (`self.Recharge Increment ULT`)) 0 100)))

(fn `CanUse`
  (returns (`Can Use` :type Boolean))
  (if (`|EnumEquality` (`self.Toggle Enum`) "NewEnumerator0")
    (set `self.tactical pre used charge` (`self.Current tactical charge`))
    (bind _result (`/Engine/EditorBlueprintResources/StandardMacros.DecrementInt` (`self.Current tactical charge`))
      (:`  `
        (set `self.Current tactical charge` (`KismetMathLibrary.Clamp` _result 0 (`self.Max tactical charge`)))
        (if (> (`self.tactical pre used charge`) 0)
          (`KismetSystemLibrary.K2_SetTimer` null "Tactical Recharge" (`self.Tactical recharge time per unit`) true)
          (return true)
          (else
            (return false)))))))

(fn `Request ULT`
  (params (`Start Offset` :type "Float (single-precision)") (`Reset On Use` :type Boolean))
  (if (== (`self.Current Charge ULT`) 100)
    (if `Reset On Use`
      (`KismetSystemLibrary.K2_SetTimer` null "Reset ULT" `Start Offset`))))

(fn `Reset ULT`
  (set `self.Current Charge ULT` 0)
  (`KismetSystemLibrary.PrintString` "Reset"))

(fn `Scale FOV`
  (params (`FOV to Scale To` :type "Float (double-precision)") (Alpha :type "Float (double-precision)"))
  (`CameraComponent.SetFieldOfView` (`/Game/Core/Blueprints/Base_Charachter.Camera` (`self.Charachter`)) (`KismetMathLibrary.Lerp` (`self.Default Camera FOV`) `FOV to Scale To` Alpha)))

(fn `Start Debug`
  (params (Value :type Text) (InText :type Text))
  (`|ExecutionSequence`
    (:`then_0`
      (`KismetSystemLibrary.PrintText` (`|FormatText` "{X} : {A}" (`KismetSystemLibrary.MakeLiteralText` Value) (`self.Current Charge ULT`)) true true (struct :`G` 0.66 :`B` 1.0 :`A` 1.0) 0.0))
    (:`then_1`
      (`KismetSystemLibrary.PrintText` (`|FormatText` "{X} : {A}" "Q" (`self.Current tactical charge`)) true true (struct :`G` 0.66 :`B` 1.0 :`A` 1.0) 0.0))))

(fn `Start Ult Timer`
  (params (Time :type "Float (single-precision)") (bLooping :type Boolean))
  (`KismetSystemLibrary.K2_SetTimer` null "Calculate ULT charges" Time bLooping))

(fn `Tactical Recharge`
  (bind _result (`/Engine/EditorBlueprintResources/StandardMacros.IncrementInt` (`self.Current tactical charge`))
    (:`  `
      (set `self.Current tactical charge` (`KismetMathLibrary.Clamp` _result 0 (`self.Max tactical charge`))))))

(fn `Toggle`
  (`/Engine/EditorBlueprintResources/StandardMacros.FlipFlop`
    (:`A`
      (set `self.Toggle Enum` "NewEnumerator0"))
    (:`B`
      (set `self.Toggle Enum` "NewEnumerator1"))))