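; BP_Weapons is a weapon pickup that shows a prompt and attaches to the player's character when interacted with.
; Ranged enter and exit events create or destroy a screen-space WBP_WeaponPickup widget component on GunMesh, reading "PICK UP".
; On interact, GunMesh snaps to the WeaponSlot of the Base_Charachter cached from player 0 at BeginPlay.
; A switch on WeaponPriority is present but unconnected.
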(event `/Game/Core/Blueprints/Data/BPI_Interaction_Interface.On Ranged Entered`
  (params (Player :type "/Game/Core/Blueprints/Base_Charachter Object Reference"))
  ;[0.0625 0.04492 0.04492] Interaction
  (`self.InteractionWidget`
    (:`then`)
    (:`else`
      (`self.Show Widget Attached` (cast `PlayerController` (`Pawn.GetController` Player) :!pure true)))))

(event `/Game/Core/Blueprints/Data/BPI_Interaction_Interface.On Ranged Exited`
  ;[0.0625 0.04492 0.04492] Interaction
  (bind _interactionwidget (`self.InteractionWidget`)
    (:`then`
      (`ActorComponent.K2_DestroyComponent` _interactionwidget))
    (:`else`)))

(event `self.ReceiveBeginPlay`
  ;[1 1 1] Refs
  (bind _asbase_charachter (cast `/Game/Core/Blueprints/Base_Charachter` (`GameplayStatics.GetPlayerCharacter` 0)))
  (set `self.Player` _asbase_charachter))

(event `/Game/Core/Blueprints/Data/BPI_Interaction_Interface.OnRangedInteract`
  (`self.AttachWeapons`))

(fn `AttachWeapons`
  (`SceneComponent.K2_AttachToComponent` (`self.Gun Mesh`) (`/Game/Core/Blueprints/Base_Charachter.WeaponSlot` (`self.Player`)) "None" "SnapToTarget" "SnapToTarget" "SnapToTarget" true))

(fn `Show Widget Attached`
  (params (OwningPlayer :type "PlayerController Object Reference"))
  (bind _returnvalue (`|CreateWidget` "/Game/Core/UI/WBP_WeaponPickup.WBP_WeaponPickup_C" OwningPlayer "PICK UP"))
  (bind _returnvalue_2 (`AddComponent|NODE_AddWidgetComponent-0`))
  (set `self.InteractionWidget` _returnvalue_2)
  (`WidgetComponent.SetWidget` _returnvalue_2 _returnvalue)
  (`WidgetComponent.SetWidgetSpace` _returnvalue_2 "Screen")
  (`WidgetComponent.SetDrawAtDesiredSize` _returnvalue_2 true)
  (`PrimitiveComponent.SetCollisionEnabled` _returnvalue_2 "NoCollision")
  (`SceneComponent.K2_AttachToComponent` _returnvalue_2 (`self.Gun Mesh`) "None" "SnapToTarget" "SnapToTarget" "SnapToTarget" true))

(fn `UserConstructionScript`)